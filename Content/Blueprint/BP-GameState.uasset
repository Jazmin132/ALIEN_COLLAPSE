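; Game state Blueprint that persists the player's last position and destroyed actors through a BP_SaveG save slot.
; On BeginPlay it binds to OnDeath on every BP_DamageableComponent, then restores the player and destroys saved actors, or creates an empty save.
; Helper functions append destroyed actors to the loaded save, delete the slot, or save position.
; SaveLastPos writes a fresh save object, discarding the stored destroyed-actor list.
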(event `self.ReceiveBeginPlay`
  (bind _outactors (`GameplayStatics.GetAllActorsOfClass` null))
  (for _array_element _outactors
    (bind _returnvalue (`self.GetComponentByClass` _array_element "/Game/Blueprint/ActorComponets/BP_DamageableComponent.BP_DamageableComponent_C"))
    (`/Engine/EditorBlueprintResources/StandardMacros.IsValid` _returnvalue
      (:`Is Valid`
        (add `/Game/Blueprint/ActorComponets/BP_DamageableComponent.OnDeath` _returnvalue (`|CreateDelegate` :!event `SaveNewDetroyedActors`)))))
  (bind _returnvalue_2 (`GameplayStatics.DoesSaveGameExist` "Save Game Yeah"))
  (if _returnvalue_2
    (bind _returnvalue_3 (`GameplayStatics.LoadGameFromSlot` "Save Game Yeah"))
    (bind _asbp_save_g (cast `/Game/Blueprint/BP_SaveG` _returnvalue_3))
    (`|ExecutionSequence`
      (:`then_0`
        (bind _lastplayerpos (`/Game/Blueprint/BP_SaveG.LastPlayerPos` _asbp_save_g))
        (if (not (== _lastplayerpos (`self.Vector 0`)))
          (`self.K2_SetActorTransform` (`GameplayStatics.GetPlayerPawn` 0) _lastplayerpos false false)))
      (:`then_1`
        (for _array_element_2 (`/Game/Blueprint/BP_SaveG.DestroyedActors` _asbp_save_g)
          (`self.K2_DestroyActor` _array_element_2))))
    (else
      (bind _returnvalue_4 (`GameplayStatics.CreateSaveGameObject` "/Game/Blueprint/BP_SaveG.BP_SaveG_C"))
      (`GameplayStatics.SaveGameToSlot` _returnvalue_4 "Save Game Yeah"))))

(fn `ClearSaveGame`
  (`GameplayStatics.DeleteGameInSlot` "Save Game Yeah"))

(fn `SaveLastPos`
  (params (LastPos :type "Transform Structure"))
  (bind _returnvalue (`GameplayStatics.CreateSaveGameObject` "/Game/Blueprint/BP_SaveG.BP_SaveG_C"))
  (`/Game/Blueprint/BP_SaveG.SetLastPlayerPos` _returnvalue LastPos)
  (`GameplayStatics.SaveGameToSlot` _returnvalue "Save Game Yeah"))

(fn `SaveNewDetroyedActors`
  (params (DestroyedActor :type "Actor Object Reference"))
  (bind _returnvalue (`GameplayStatics.DoesSaveGameExist` "Save Game Yeah"))
  (if _returnvalue
    (bind _returnvalue_2 (`GameplayStatics.LoadGameFromSlot` "Save Game Yeah"))
    (bind _asbp_save_g (cast `/Game/Blueprint/BP_SaveG` _returnvalue_2))
    (`/Game/Blueprint/BP_SaveG.AddDestroyedActors` _asbp_save_g DestroyedActor)
    (`GameplayStatics.SaveGameToSlot` _asbp_save_g "Save Game Yeah")))

(fn `UserConstructionScript`)