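; Turret-style enemy that turns toward the player and fires projectiles while the player is within range.
; Range and fire interval load from DT_EnemiesData by enemy type.
; A looping 0.016-second timer checks distance, eases rotation toward the player and toggles M_Blink's blink, recreating its dynamic material each pass.
; A second timer spawns BP_EnemyPorjectile aimed at the player when rotation is allowed.
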(event `self.ReceiveBeginPlay`
  (`self.LoadValues`)
  (set `self.ParamValue` 0.0)
  (`|ExecutionSequence`
    (:`then_0`
      (set `self.Current HP` (`self.MaxHP`)))
    (:`then_1`
      (bind _asbp_first_person_character (cast `/Game/FirstPerson/Blueprints/BP_FirstPersonCharacter` (`GameplayStatics.GetPlayerCharacter` 0)))
      (set `self.FP_Character` _asbp_first_person_character)
      (`KismetSystemLibrary.K2_SetTimerDelegate` (delegate `Should Rotate`) 0.016 true)
      (`KismetSystemLibrary.K2_SetTimerDelegate` (delegate `Fire to player`) (`self.Time`) true))))

(event `Fire to player`
  (if (`self.Rotate Allowed`)
    (`|SpawnActorFromClass` "/Game/FirstPerson/Blueprints/BP_EnemyPorjectile.BP_EnemyPorjectile_C" (`KismetMathLibrary.MakeTransform` (`SceneComponent.K2_GetComponentLocation` (`self.Spawn Bala`)) (`KismetMathLibrary.FindLookAtRotation` (`self.K2_GetActorLocation`) (`self.K2_GetActorLocation` (`self.FP_Character`)))) "Undefined" "OverrideRootScale" null null)))

(event `Face Player`
  (bind (_returnvalue_roll _returnvalue_pitch _returnvalue_yaw) (`KismetMathLibrary.BreakRotator` (`KismetMathLibrary.RInterpTo` (`self.K2_GetActorRotation`) (`KismetMathLibrary.FindLookAtRotation` (`self.K2_GetActorLocation`) (`self.K2_GetActorLocation` (`self.FP_Character`))) (`GameplayStatics.GetWorldDeltaSeconds`) 2.0)))
  ;[1 1 1] Siempre mira al jugador
  (if (`self.Rotate Allowed`)
    (`self.K2_SetActorRotation` (`KismetMathLibrary.MakeRotator` _returnvalue_roll _returnvalue_pitch _returnvalue_yaw))
    (else
      (`self.Should Rotate`))))

(event `Should Rotate`
  ;[1 1 1] Se fija si deberia rotar
  (if (< (`self.GetDistanceTo` (`self.FP_Character`)) (`self.Distance`))
    (set `self.Rotate Allowed` true)
    (set `self.ParamValue` 1.0)
    (`self.Change Param`)
    (`self.Face Player`)
    (else
      (set `self.Rotate Allowed` false)
      (set `self.ParamValue` 0.0)
      (`self.Change Param`))))

(event `Change Param`
  (bind _cube1 (`self.Cube1`))
  (bind _returnvalue (`KismetMaterialLibrary.CreateDynamicMaterialInstance` "/Game/Blueprint/Materials/M_Blink.M_Blink"))
  (bind _output_get (set `self.Material` _returnvalue))
  (`PrimitiveComponent.SetMaterial` _cube1 0 _output_get)
  (`MeshComponent.SetScalarParameterValueOnMaterials` _cube1 "BlinkActivate" (`self.ParamValue`)))

(fn `LoadValues`
  (bind _returnvalue (`|GetDataTableRow` "/Game/Blueprint/FacePlayer/DT_EnemiesData.DT_EnemiesData" (`KismetStringLibrary.Conv_StringToName` (`|GetEnumeratorNameAsString` (`self.Type_FaceP`))))
    (:`then`
      (bind (_distance _time) (break `/Game/Blueprint/FEnemyData` _returnvalue))
      (set `self.Distance` _distance)
      (set `self.Time` _time))))

(fn `UserConstructionScript`)