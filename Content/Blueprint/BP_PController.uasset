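; BP_PController is a player controller that manages the health widget and the win and lose screens.
; BeginPlay hides the cursor and creates WBP_Health, which UpdatePoints later feeds with current and maximum points.
; On possess, it binds to the pawn's BP_DamageableComponent OnDamage event, provided the HUD is a BP_HUD.
; ActivateWin and ActivateLose pause the game, show the cursor and display their respective widgets.
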(event `self.ReceiveBeginPlay`
  (set `self.bShowMouseCursor` false)
  (bind _returnvalue (`|CreateWidget` "/Game/Blueprint/UI-WBP/WBP_Health.WBP_Health_C"))
  (bind _output_get (set `self.WP_Health` _returnvalue))
  (`UserWidget.AddToViewport` _output_get 0))

(event `self.ReceivePossess`
  (params (PossessedPawn :type "Pawn Object Reference"))
  (bind _returnvalue (`self.GetComponentByClass` PossessedPawn "/Game/Blueprint/ActorComponets/BP_DamageableComponent.BP_DamageableComponent_C"))
  (`/Engine/EditorBlueprintResources/StandardMacros.IsValid` _returnvalue
    (:`Is Valid`
      (bind _asbp_hud (cast `/Game/Blueprint/BP_HUD` (`self.GetHUD`)))
      (add `/Game/Blueprint/ActorComponets/BP_DamageableComponent.OnDamage` _returnvalue (`|CreateDelegate` _asbp_hud :!event `DisplayNewLife`)))))

(event `Update Points`
  (params (`Current Points` :type "Float (double-precision)") (MaxPoints :type "Float (double-precision)"))
  (`/Game/Blueprint/UI-WBP/WBP_Health.Set Points Info` (`self.WP_Health`) `Current Points` MaxPoints))

(event `ActivateLose`
  (`GameplayStatics.SetGamePaused` true)
  (set `self.bShowMouseCursor` true)
  (bind _returnvalue (`|CreateWidget` "/Game/Blueprint/UI-WBP/WBP_LOSE.WBP_LOSE_C"))
  (`UserWidget.AddToViewport` _returnvalue 0))

(event `ActivateWin`
  (`GameplayStatics.SetGamePaused` true)
  (set `self.bShowMouseCursor` true)
  (bind _returnvalue (`|CreateWidget` "/Game/Blueprint/UI-WBP/WBP_Win.WBP_Win_C"))
  (`UserWidget.AddToViewport` _returnvalue 0))

(fn `UserConstructionScript`)