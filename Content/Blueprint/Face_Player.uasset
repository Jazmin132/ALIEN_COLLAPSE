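; Turret-like actor that turns to face the first-person player within close range and shoots projectiles at them.
; BeginPlay caches the character and starts ShouldRotate, which re-polls distance through a tiny looping Delay rather than Tick or a timer.
; In range, each poll calls FacePlayer to interpolate toward a look-at rotation, and Firetoplayer, whose Delay acts as cooldown before spawning BP_FirstPersonProjectile at SpawnBala aimed at the player.
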(event `self.ReceiveBeginPlay`
  (`|ExecutionSequence`
    (:`then_0`
      (bind _asbp_first_person_character (cast `/Game/FirstPerson/Blueprints/BP_FirstPersonCharacter` (`GameplayStatics.GetPlayerCharacter` 0)))
      (set `self.FP_Character` _asbp_first_person_character)
      (`self.Should Rotate`))))

(event `Face Player`
  (bind (_returnvalue_roll _returnvalue_pitch _returnvalue_yaw) (`KismetMathLibrary.BreakRotator` (`KismetMathLibrary.RInterpTo` (`self.K2_GetActorRotation`) (`KismetMathLibrary.FindLookAtRotation` (`self.K2_GetActorLocation`) (`self.K2_GetActorLocation` (`self.FP_Character`))) (`GameplayStatics.GetWorldDeltaSeconds`) 20.0)))
  ;[1 1 1] Siempre mira al jugador
  (if (`self.Rotate Allowed`)
    (`self.K2_SetActorRotation` (`KismetMathLibrary.MakeRotator` _returnvalue_roll _returnvalue_pitch _returnvalue_yaw))
    (else
      (`self.Should Rotate`))))

(event `Fire to player`
  ;[1 1 1] Hacer con un evento TICK EL COOLDOWN DEL DISPARO
  (`KismetSystemLibrary.Delay` 3.0)
  (`|SpawnActorFromClass` "/Game/FirstPerson/Blueprints/BP_FirstPersonProjectile.BP_FirstPersonProjectile_C" (`KismetMathLibrary.MakeTransform` (`SceneComponent.K2_GetComponentLocation` (`self.Spawn Bala`)) (`KismetMathLibrary.FindLookAtRotation` (`self.K2_GetActorLocation`) (`self.K2_GetActorLocation` (`self.FP_Character`)))) "Undefined" "OverrideRootScale" null null))

(event `Should Rotate`
  ;[1 1 1] Se fija si deberia rotar
  (if (< (`self.GetDistanceTo` (`self.FP_Character`)) 350.0)
    (set `self.Rotate Allowed` true)
    (`self.Face Player`)
    (`|ExecutionSequence`
      (:`then_0`
        ;;[1 1 1] Cambiar a timer mas adelante
        (`KismetSystemLibrary.Delay` 0.001 :!label _label)
        (`self.Should Rotate`))
      (:`then_1`
        (`self.Fire to player`)))
    (else
      (set `self.Rotate Allowed` false)
      (goto _label))))

(fn `UserConstructionScript`)