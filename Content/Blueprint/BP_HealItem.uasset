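; Healing pickup that restores health to any actor with a BP_DamageableComponent overlapping Sphere1.
; On pickup it calls OnHealing with the Healing amount, plays a sound and destroys itself.
; A separate CollisionShader volume switches on a hologram effect when the first-person character enters, creating a dynamic MHologram material on Sphere and setting "Activate".
; Leaving that volume only resets the stored ParamValue, without updating the material.
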(event `self.Sphere1.OnComponentBeginOverlap`
  (params (OverlappedComponent :type "PrimitiveComponent Object Reference") (OtherActor :type "Actor Object Reference") (OtherComp :type "PrimitiveComponent Object Reference") (OtherBodyIndex :type Integer) (bFromSweep :type Boolean) (SweepResult :type "HitResult Structure (by ref)"))
  (bind _returnvalue (`self.GetComponentByClass` OtherActor "/Game/Blueprint/ActorComponets/BP_DamageableComponent.BP_DamageableComponent_C"))
  (`/Engine/EditorBlueprintResources/StandardMacros.IsValid` _returnvalue
    (:`Is Valid`
      (`/Game/Blueprint/ActorComponets/BP_DamageableComponent.OnHealing` _returnvalue (`self.Healing`))
      (`GameplayStatics.PlaySoundAtLocation` "/Game/Blueprint/Sounds/RecuperarVida.RecuperarVida" (`self.K2_GetActorLocation`) (struct) 1.0 1.0 0.0 null null null null)
      (`self.K2_DestroyActor`))))

(event `self.ReceiveBeginPlay`
  ;[1 1 1] SET PARAM HOLOGRAM
  (set `self.Param Value` 0.0))

(event `self.CollisionShader.OnComponentBeginOverlap`
  (params (OverlappedComponent :type "PrimitiveComponent Object Reference") (OtherActor :type "Actor Object Reference") (OtherComp :type "PrimitiveComponent Object Reference") (OtherBodyIndex :type Integer) (bFromSweep :type Boolean) (SweepResult :type "HitResult Structure (by ref)"))
  ;[1 1 1] SET PARAM HOLOGRAM
  (cast `/Game/FirstPerson/Blueprints/BP_FirstPersonCharacter` OtherActor)
  (set `self.Param Value` 1.0)
  (bind _returnvalue (`KismetMaterialLibrary.CreateDynamicMaterialInstance` "/Game/Blueprint/Materials/M-Hologram.M-Hologram"))
  (bind _output_get (set `self.Material` _returnvalue))
  (`PrimitiveComponent.SetMaterial` (`self.Sphere`) 0 _output_get)
  (`MeshComponent.SetScalarParameterValueOnMaterials` (`self.Sphere`) "Activate" (`self.Param Value`)))

(event `self.CollisionShader.OnComponentEndOverlap`
  (params (OverlappedComponent :type "PrimitiveComponent Object Reference") (OtherActor :type "Actor Object Reference") (OtherComp :type "PrimitiveComponent Object Reference") (OtherBodyIndex :type Integer))
  ;[1 1 1] SET PARAM HOLOGRAM
  (cast `/Game/FirstPerson/Blueprints/BP_FirstPersonCharacter` OtherActor)
  (set `self.Param Value` 0.0))

(fn `UserConstructionScript`)