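; BP_DamageableComponent is an actor component that gives its owner hit points, damage and death handling, for both the player and other actors.
; GetDamage clamps HP, broadcasts through OnDamage, plays the Lose sound on every hit, and calls OnDeath at zero.
; Death activates the lose state on BP_PController for the player; other owners award points to the player and are destroyed with a sound.
; Healing is player-only and unclamped.
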(event `self.ReceiveBeginPlay`
  (bind _output_get (set `self.CurrentHP` (`self.MaxHP`)))
  (`self.OnDamage` 0.0 _output_get))

(fn `GetDamage`
  (params (Damage :type "Float (double-precision)"))
  (bind _returnvalue (`GameplayStatics.GetPlayerPawn` 0))
  (bind _returnvalue_2 (`self.GetOwner`))
  (bind _output_get (set `self.CurrentHP` (`KismetMathLibrary.FClamp` (- (`self.CurrentHP`) Damage) 0.0 (`self.MaxHP`))))
  (`self.OnDamage` Damage _output_get)
  (`GameplayStatics.PlaySoundAtLocation` "/Game/Blueprint/Sounds/Lose.Lose" (`Actor.K2_GetActorLocation` (`self.GetOwner`)) (struct) 1.0 1.0 0.0 null null null null)
  (if (== _output_get 0.0)
    (`self.OnDeath` (`self.GetOwner`))
    (if (`self.IsPlayer`)
      (bind _asbp_first_person_character (cast `/Game/FirstPerson/Blueprints/BP_FirstPersonCharacter` _returnvalue))
      (bind _asbp_pcontroller (cast `/Game/Blueprint/BP_PController` (`Pawn.GetController` _asbp_first_person_character)))
      (`/Game/Blueprint/BP_PController.ActivateLose` _asbp_pcontroller)
      (else
        (bind _asbp_first_person_character_2 (cast `/Game/FirstPerson/Blueprints/BP_FirstPersonCharacter` _returnvalue))
        (`/Game/FirstPerson/Blueprints/BP_FirstPersonCharacter.GetPoints` _asbp_first_person_character_2 (`self.Points`))
        (`GameplayStatics.PlaySoundAtLocation` "/Game/Blueprint/Sounds/DetruirCarton.DetruirCarton" (`Actor.K2_GetActorLocation` _returnvalue_2) (struct) 1.0 1.0 0.0 null null null null)
        (`Actor.K2_DestroyActor` _returnvalue_2)))))

(fn `OnHealing`
  (params (HealAmount :type "Float (double-precision)"))
  (if (`self.IsPlayer`)
    (bind _output_get (set `self.CurrentHP` (+ HealAmount (`self.CurrentHP`))))
    (`self.OnHeal` _output_get)))