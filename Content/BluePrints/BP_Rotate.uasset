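; BP_Rotate is an interactable actor that rotates a set of referenced objects when the player triggers it.
; At BeginPlay it applies an initial rotation offset to every actor in its Objects array through the shared Rotate function.
; The Collider_2 overlap enables input only while the first-person character is inside, and each Interact press adds a fixed local rotation step to those actors.
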(event `self.ReceiveActorBeginOverlap`
  (params (OtherActor :type "Actor Object Reference")))

(event `self.ReceiveBeginPlay`
  (`self.Rotate` (`self.NewRotation`)))

(event `self.Collider_2.OnComponentBeginOverlap`
  (params (OverlappedComponent :type "PrimitiveComponent Object Reference") (OtherActor :type "Actor Object Reference") (OtherComp :type "PrimitiveComponent Object Reference") (OtherBodyIndex :type Integer) (bFromSweep :type Boolean) (SweepResult :type "HitResult Structure (by ref)"))
  (cast `/Game/FirstPerson/Blueprints/BP_FirstPersonCharacter` OtherActor)
  (`self.EnableInput` (`GameplayStatics.GetPlayerController` 0)))

(event `InputAction|Interact`
  (params (Key :type "Key Structure"))
  (:`Pressed`
    (`self.Rotate` (struct :`Pitch` 30.0 :`Yaw` 10.0))))

(event `self.Collider_2.OnComponentEndOverlap`
  (params (OverlappedComponent :type "PrimitiveComponent Object Reference") (OtherActor :type "Actor Object Reference") (OtherComp :type "PrimitiveComponent Object Reference") (OtherBodyIndex :type Integer))
  (cast `/Game/FirstPerson/Blueprints/BP_FirstPersonCharacter` OtherActor)
  (`self.DisableInput` (`GameplayStatics.GetPlayerController` 0)))

(fn `Rotate`
  (params (Rotation :type "Rotator Structure"))
  (for _array_element (`self.Objects`)
    (`self.K2_AddActorLocalRotation` _array_element Rotation false false))
  (return))

(fn `UserConstructionScript`)