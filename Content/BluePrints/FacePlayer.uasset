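; FacePlayer is an actor Blueprint that keeps turning itself to look at the first-person player character.
; On BeginPlay it casts and caches the player as BP_FirstPersonCharacter, then starts the FacePlayer event.
; That event interpolates the actor's full rotation toward a look-at rotation at the player's location.
; It loops by calling itself after a short Delay instead of using Tick, while still interpolating with world delta seconds.
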(event `self.ReceiveBeginPlay`
  (`|ExecutionSequence`
    (:`then_0`
      (bind _asbp_first_person_character (cast `/Game/FirstPerson/Blueprints/BP_FirstPersonCharacter` (`GameplayStatics.GetPlayerCharacter` 0)))
      (set `self.As BP First Person Character` _asbp_first_person_character)
      (`self.FacePlayer`))))

(event `FacePlayer`
  (bind (_returnvalue_roll _returnvalue_pitch _returnvalue_yaw) (`KismetMathLibrary.BreakRotator` (`KismetMathLibrary.RInterpTo` (`self.K2_GetActorRotation`) (`KismetMathLibrary.FindLookAtRotation` (`self.K2_GetActorLocation`) (`self.K2_GetActorLocation` (`self.As BP First Person Character`))) (`GameplayStatics.GetWorldDeltaSeconds`) 20.0)))
  ;[1 1 1] Mirar al jugador
  (`self.K2_SetActorRotation` (`KismetMathLibrary.MakeRotator` _returnvalue_roll _returnvalue_pitch _returnvalue_yaw))
  (`KismetSystemLibrary.Delay` 0.01) ; El delay es para darle tiempo al codigo para terminar y se llame otra vez
  (`self.FacePlayer`))

(fn `UserConstructionScript`)