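; Enemy character that detects the first-person player and provides events to turn toward and shoot them.
; AI perception writes the sensed state and target actor to the Blackboard, with a note pointing to a decorator check in BT_Enemy.
; Rotate_To_Player smoothly interpolates toward the player cached at BeginPlay.
; Shoot_Player plays a gun animation and fire sound, spawning a projectile at the Billboard aimed along the actor-to-player direction.
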(event `self.AIPerception.OnTargetPerceptionUpdated`
  (params (Actor :type "Actor Object Reference") (Stimulus :type "AIStimulus Structure"))
  (bind _returnvalue (`AIBlueprintHelperLibrary.GetBlackboard` (`self.GetController`)))
  (bind _asbp_first_person_character (cast `/Game/FirstPerson/Blueprints/BP_FirstPersonCharacter` Actor))
  (`BlackboardComponent.SetValueAsBool` _returnvalue "IsPlayerSight" (`.bSuccessfullySensed` (break `AIStimulus` Stimulus)))
  (`BlackboardComponent.SetValueAsObject` _returnvalue "TargetActor" _asbp_first_person_character))

(event `self.ReceiveBeginPlay`
  (bind _asbp_first_person_character (cast `/Game/FirstPerson/Blueprints/BP_FirstPersonCharacter` (`GameplayStatics.GetPlayerCharacter` 0)))
  (set `self.As BP First Person Character` _asbp_first_person_character))

(event `Rotate_To_Player`
  (bind (_returnvalue_roll _returnvalue_pitch _returnvalue_yaw) (`KismetMathLibrary.BreakRotator` (`KismetMathLibrary.RInterpTo` (`self.K2_GetActorRotation`) (`KismetMathLibrary.FindLookAtRotation` (`self.K2_GetActorLocation`) (`self.K2_GetActorLocation` (`self.As BP First Person Character`))) (`GameplayStatics.GetWorldDeltaSeconds`) 2.0)))
  ;[1 1 1] Always Rotate
  (`self.K2_SetActorRotation` (`KismetMathLibrary.MakeRotator` _returnvalue_roll _returnvalue_pitch _returnvalue_yaw)))

(event `Shoot_Player`
  ;[1 1 1] Shoot at Player
  (`SkeletalMeshComponent.PlayAnimation` (`self.Mesh`) "/Game/Enemy/Gunplay.Gunplay" false)
  (`|SpawnActorFromClass` "/Game/FirstPerson/Blueprints/BP_EnemyPorjectile.BP_EnemyPorjectile_C" (`KismetMathLibrary.MakeTransform` (`SceneComponent.K2_GetComponentLocation` (`self.Billboard`)) (`KismetMathLibrary.FindLookAtRotation` (`self.K2_GetActorLocation`) (`self.K2_GetActorLocation` (`self.As BP First Person Character`)))) "Undefined" "OverrideRootScale" null null)
  (`GameplayStatics.PlaySoundAtLocation` "/Game/FPWeapon/Audio/FirstPersonTemplateWeaponFire02.FirstPersonTemplateWeaponFire02" (`self.K2_GetActorLocation`) (struct) 1.0 1.0 0.0 null null null null))

(fn `UserConstructionScript`)